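; Scoreboard actor that displays an arithmetic operation as two operands, an operator symbol and the result.
; UpdateBoard computes add, subtract, multiply or divide from its inputs and writes all four texts, with no divide-by-zero check visible.
; ClearBoard resets the texts to placeholders.
; Every Tick, the actor sets its yaw from the player character mesh's yaw plus a fixed offset, so it turns with the player.
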(event `self.ReceiveTick`
  (params (DeltaSeconds :type "Float (single-precision)"))
  (`|ExecutionSequence`
    (:`then_0`
      (`self.K2_SetActorRotation` (`KismetMathLibrary.MakeRotator` 0.0 0.0 (+ (.yaw (`SceneComponent.K2_GetComponentRotation` (`Character.Mesh` (`GameplayStatics.GetPlayerCharacter` 0)))) 270.0))))))

(fn `ClearBoard`
  (`TextRenderComponent.K2_SetText` (`self.Sum`) (`KismetTextLibrary.Conv_StringToText` "0"))
  (`TextRenderComponent.K2_SetText` (`self.Operation`) (`KismetTextLibrary.Conv_StringToText` ""))
  (`TextRenderComponent.K2_SetText` (`self.Num_1`) (`KismetTextLibrary.Conv_StringToText` "-"))
  (`TextRenderComponent.K2_SetText` (`self.Num_2`) (`KismetTextLibrary.Conv_StringToText` "-")))

(fn `UpdateBoard`
  (params (num1 :type Integer) (num2 :type Integer) (op :type "/Game/Blueprints/Scoreboard/EOperation Enum"))
  (locals (total :type Integer) (operationTxt :type Text))
  (`|ExecutionSequence`
    (:`then_0`
      (switch `/Game/Blueprints/Scoreboard/EOperation` op
        (:`NewEnumerator0`
          (set `local.total` (+ num1 num2))
          (set `local.operationTxt` "+"))
        (:`NewEnumerator1`
          (set `local.total` (- num1 num2))
          (set `local.operationTxt` "-"))
        (:`NewEnumerator2`
          (set `local.total` (* num1 num2))
          (set `local.operationTxt` "X"))
        (:`NewEnumerator3`
          (set `local.total` (/ num1 num2))
          (set `local.operationTxt` "/"))))
    (:`then_1`
      (`TextRenderComponent.K2_SetText` (`self.Sum`) (`KismetTextLibrary.Conv_StringToText` (`KismetStringLibrary.Conv_IntToString` (`local.total`))))
      (`TextRenderComponent.K2_SetText` (`self.Operation`) (`local.operationTxt`))
      (`TextRenderComponent.K2_SetText` (`self.Num_1`) (`KismetTextLibrary.Conv_StringToText` (`KismetStringLibrary.Conv_IntToString` num1)))
      (`TextRenderComponent.K2_SetText` (`self.Num_2`) (`KismetTextLibrary.Conv_StringToText` (`KismetStringLibrary.Conv_IntToString` num2))))))

(fn `UserConstructionScript`)