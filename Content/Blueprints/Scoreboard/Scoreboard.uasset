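; Scoreboard actor that shows the match score and timer in the world, turning each Tick to follow the player mesh's yaw with a fixed offset.
; It polls InGameGameMode every frame for score and time, formatting time as minutes and zero-padded seconds.
; The GameActive flag switches the cube between glass and black materials and reveals FinalScoreTxt when play is inactive, while the timer stays visible.
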(event `self.ReceiveTick`
  (params (DeltaSeconds :type "Float (single-precision)"))
  (bind _timertxt (`self.TimerTxt`))
  (bind _cube (`self.Cube`))
  (`|ExecutionSequence`
    (:`then_0`
      (`self.K2_SetActorRotation` (`KismetMathLibrary.MakeRotator` 0.0 0.0 (+ (.yaw (`SceneComponent.K2_GetComponentRotation` (`Character.Mesh` (`GameplayStatics.GetPlayerCharacter` 0)))) 270.0))))
    (:`then_1`
      (bind _asin_game_game_mode (cast `/Game/Blueprints/GameMode/InGameGameMode` (`GameplayStatics.GetGameMode`)))
      (bind _score (`/Game/Blueprints/GameMode/InGameGameMode.GetScore` _asin_game_game_mode))
      (`TextRenderComponent.K2_SetText` (`self.ScoreTxt`) (`KismetTextLibrary.Conv_IntToText` _score))
      (bind _time (`/Game/Blueprints/GameMode/InGameGameMode.GetTime` _asin_game_game_mode))
      (bind _returnvalue (mod _time 60))
      (if (< _returnvalue 10)
        (bind _returnvalue_2 (`KismetStringLibrary.Conv_IntToString` (/ _time 60)))
        (bind _returnvalue_3 (`KismetStringLibrary.Conv_IntToString` _returnvalue))
        (`TextRenderComponent.K2_SetText` _timertxt (`KismetTextLibrary.Conv_StringToText` (`KismetStringLibrary.Concat_StrStr` _returnvalue_2 ":" "0" _returnvalue_3)))
        (else
          (`TextRenderComponent.K2_SetText` _timertxt (`KismetTextLibrary.Conv_StringToText` (`KismetStringLibrary.Concat_StrStr` _returnvalue_2 ":" _returnvalue_3))))))
    (:`then_2`
      (bind _asin_game_game_mode_2 (cast `/Game/Blueprints/GameMode/InGameGameMode` (`GameplayStatics.GetGameMode`)))
      (if (`/Game/Blueprints/GameMode/InGameGameMode.gameActive` _asin_game_game_mode_2)
        (`SceneComponent.SetVisibility` (`self.FinalScoreTxt`) false false)
        (`SceneComponent.SetVisibility` (`self.TimerTxt`) true true)
        (`PrimitiveComponent.SetMaterial` _cube 0 "/Game/StarterContent/Materials/Glass_Mat.Glass_Mat")
        (else
          (`SceneComponent.SetVisibility` (`self.FinalScoreTxt`) true true)
          (`SceneComponent.SetVisibility` (`self.TimerTxt`) true false)
          (`PrimitiveComponent.SetMaterial` _cube 0 "/Game/StarterContent/Materials/Colours/Black_Mat.Black_Mat"))))))

(fn `UserConstructionScript`)