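; MapSelect is a gamepad-controlled character or pawn, named for map selection, that moves and turns its view with the sticks.
; Left stick axes feed AddMovementInput along the Camera component's right and forward vectors, so movement follows the view.
; Right stick X adds world rotation to the Camera using a vector scaled by the raw axis value, without delta time.
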(event `InputAxisKey|Gamepad_LeftX`
  (params (AxisValue :type "Float (single-precision)"))
  (`self.AddMovementInput` (`SceneComponent.GetRightVector` (`self.Camera`)) AxisValue))

(event `InputAxisKey|Gamepad_RightX`
  (params (AxisValue :type "Float (single-precision)"))
  (`SceneComponent.K2_AddWorldRotation` (`self.Camera`) (* (struct :`Yaw` 1.0) AxisValue) false false))

(event `InputAxisKey|Gamepad_LeftY`
  (params (AxisValue :type "Float (single-precision)"))
  (`self.AddMovementInput` (`SceneComponent.GetForwardVector` (`self.Camera`)) AxisValue))

(fn `UserConstructionScript`)